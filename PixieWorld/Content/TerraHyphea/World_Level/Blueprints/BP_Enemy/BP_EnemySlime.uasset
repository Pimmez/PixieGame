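; Slime enemy that flags sighting of the Aria player character on its AI blackboard and drops loot when killed.
; PawnSensing sets the "HasSeenPlayer?" key; AnyDamage reduces Health, spawning a gravity-enabled B_ChildJelly before destroying the slime.
; FollowPlayer moves to the player and plays an attack animation, but its in-file caller is disconnected.
; Sight-flag updates, attack montage, cooldown and damage dealing are also unwired leftovers.
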(event OnSeePawn(PawnSensing)
  (params (Pawn :type Pawn%20Object%20Reference))
  (Utilities|Casting|CastToBP_AriaCharacter2 Pawn)
  (AI|Components|Blackboard|SetValueasBool (AI|GetBlackboard (AI|GetAIController self)) (Utilities|Name|MakeLiteralName "HasSeenPlayer?") true))

(event Custom|FollowPlayer
  ;[1 1 1] Follow Player -> Attack
  (Variables|Default|SetCanAttack true)
  (if (Variables|Default|GetIsPlayerInSight?)
    (AI|AIMoveTo self "0, 0, 0" (Game|Player|GetPlayerPawn 0) 2e+02 false
      (:OnSuccess
        (if (Variables|Default|GetCanAttack)
          (Variables|Default|SetCanAttack false)
          ;[1 1 1] Attack State
          (Components|Animation|PlayAnimation (Variables|Character|GetMesh) "/Game/TerraHyphea/Art/3D/Slime/Animations/Slime_Attack_Anim.Slime_Attack_Anim" false))))))

(event Game|Damage|EventAnyDamage
  (params (Damage :type Float%20%28single-precision%29) (DamageType :type Damage%20Type%20Object%20Reference) (InstigatedBy :type Controller%20Object%20Reference) (DamageCauser :type Actor%20Object%20Reference))
  ;[1 1 1] Apply Damage
  (bind _output_get (Variables|Default|SetHealth (- (Variables|Default|GetHealth) Damage)))
  (if (<= _output_get 0.0)
    ;[1 1 1] Spawn Item (Loot)
    (bind _returnvalue (Game|SpawnActorfromClass "/Game/TerraHyphea/World_Level/Blueprints/Pickup_Items/B_ChildJelly.B_ChildJelly_C" (Math|Conversions|ToTransform(Vector) (Transformation|GetActorLocation)) "Undefined" 0 0))
    (Physics|SetEnableGravity (Variables|/Game/TerraHyphea/World_Level/Blueprints/Pickup_Items/B_ItemPickupParent.B_ItemPickupParent_C|GetStaticMesh _returnvalue) true)
    (Actor|DestroyActor)))

(fn ConstructionScript)