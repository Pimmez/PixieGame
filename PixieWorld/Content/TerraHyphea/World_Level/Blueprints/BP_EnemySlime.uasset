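; BP_EnemySlime is an enemy slime that chases and damages what it sees, then drops loot on death.
; PawnSensing stores the seen pawn and starts an AI move toward player controller 0, applying damage to that pawn when the move succeeds.
; Incoming damage reduces Health; at zero it spawns a gravity-enabled B_ChildJelly and destroys itself.
; The sight flag is never cleared beforehand, so the stop-movement branch is effectively unused.
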(event OnSeePawn(PawnSensing)
  (params (Pawn :type Pawn%20Object%20Reference))
  ;[1 1 1] On See Pawn -> Follow Player
  (Variables|Default|SetPawn Pawn)
  (Variables|Default|SetIsPlayerInSight? true)
  (CallFunction|FollowPlayer))

(event Custom|FollowPlayer
  ;[1 1 1] Follow Player -> Attack
  (if (Variables|Default|GetIsPlayerInSight?)
    (AI|AIMoveTo self "0, 0, 0" (Game|GetPlayerController 0) 2e+02 false
      (:OnSuccess
        (CallFunction|Attack)))
    (else
      (Variables|Default|SetIsPlayerInSight? false)
      (Components|Movement|StopMovementImmediately (Variables|Character|GetCharacterMovement)))))

(event Custom|Attack
  ;[1 1 1] Attack State
  (Development|PrintString "Slap, Hit, Attack")
  (Game|Damage|ApplyDamage (Variables|Default|GetPawn) 1e+01 0 0))

(event Game|Damage|EventAnyDamage
  (params (Damage :type Float%20%28single-precision%29) (DamageType :type Damage%20Type%20Object%20Reference) (InstigatedBy :type Controller%20Object%20Reference) (DamageCauser :type Actor%20Object%20Reference))
  ;[1 1 1] Apply Damage
  (bind _output_get (Variables|Default|SetHealth (- (Variables|Default|GetHealth) Damage)))
  (if (<= _output_get 0.0)
    ;[1 1 1] Spawn Item (Loot)
    (bind _returnvalue (Game|SpawnActorfromClass "/Game/TerraHyphea/World_Level/Blueprints/PickUp_Items/B_ChildJelly.B_ChildJelly_C" (Math|Conversions|ToTransform(Vector) (Transformation|GetActorLocation)) "Undefined" 0 0))
    (Physics|SetEnableGravity (Variables|/Game/TerraHyphea/World_Level/Blueprints/PickUp_Items/B_ItemPickupParent.B_ItemPickupParent_C|GetStaticMesh _returnvalue) true)
    (Actor|DestroyActor)))

(fn ConstructionScript)