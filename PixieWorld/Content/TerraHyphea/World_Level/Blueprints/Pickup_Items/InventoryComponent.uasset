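; Actor component that stores an inventory as a map of items to quantities, with add, query and remove functions.
; Adding sums onto the stored count, clamped to a fixed range.
; Querying returns the count and succeeds only if the item exists and the requested quantity is at least that count.
; Removal relies on that query and writes back the unclamped difference, so successful removals leave zero or negative counts.
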(event EventBeginPlay)

(event EventTick
  (params (DeltaSeconds :type Float%20%28single-precision%29)))

(fn AddtoInventory
  (params (Item%20To%20Be%20Added :type B%20Item%20Pickup%20Parent%20Class%20Reference) (Quantity :type Integer))
  (Utilities|Map|Add (Variables|Default|GetInventory) Item%20To%20Be%20Added (Math|Integer|Clamp(Integer) (+ (.Value (Utilities|Map|Find (Variables|Default|GetInventory) Item%20To%20Be%20Added)) Quantity) 0 99))
  (return true))

(fn QueryfromInventory
  (params (Item :type B%20Item%20Pickup%20Parent%20Class%20Reference) (Quantity :type Integer))
  (bind _inventory (Variables|Default|GetInventory))
  (bind (_value _returnvalue) (Utilities|Map|Find _inventory Item))
  (if (and (>= Quantity _value) _returnvalue)
    (return _value true)
    (else
      (return _value false))))

(fn RemovefromInventory
  (params (Item%20To%20Be%20Removed :type B%20Item%20Pickup%20Parent%20Class%20Reference) (Quanitity :type Integer))
  (bind (_output_quanitity _succes) (CallFunction|QueryfromInventory Item%20To%20Be%20Removed Quanitity))
  (if _succes
    (Utilities|Map|Add (Variables|Default|GetInventory) Item%20To%20Be%20Removed (- _output_quanitity Quanitity))
    (return true)
    (else
      (return false))))