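; Base pickup item actor that the player character can collect into an inventory with the Interact input.
; Overlap enables input, opens a gate and passes the item to the character's information-name display, while leaving reverses this.
; Interacting adds the item's class to the inventory and, on success, refreshes the bag widget, plays an FMOD sound and destroys the actor.
; Physics is optional, and a push event launches the mesh along the camera's forward direction with gravity enabled.
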(event Collision|EventActorBeginOverlap
  (params (OtherActor :type Actor%20Object%20Reference))
  (Input|EnableInput (Game|GetPlayerController 0))
  (bind _asbp_aria_character_2 (Utilities|Casting|CastToBP_AriaCharacter2 OtherActor))
  (Variables|Default|SetESlate_Visibility "Visible")
  (Default|GetInformationName _asbp_aria_character_2 (Variables|Default|GetActorReference))
  (Utilities|FlowControl|Gate true) ; enters at Open
)

(event EventTick
  (params (DeltaSeconds :type Float%20%28single-precision%29)))

(event EventPushPickupItemsAway
  (bind _returnvalue (Game|GetPlayerCameraManager 0))
  (bind _staticmesh (Variables|Default|GetStaticMesh))
  (bind _returnvalue_2 (Camera|GetCameraRotation _returnvalue))
  (bind _returnvalue_3 (Math|Vector|GetForwardVector _returnvalue_2))
  (Class|PrimitiveComponent|AddVelocityChangeImpulseatLocation _staticmesh (* _returnvalue_3 2.5e+02) (+ (Transformation|GetActorLocation) (* _returnvalue_3 "15.000000,0,0")) "None")
  (Physics|SetEnableGravity _staticmesh true))

(event EventBeginPlay
  (Variables|Default|SetActorReference self)
  (Physics|SetSimulatePhysics (Variables|Default|GetStaticMesh) (Variables|Default|GetisSimulatePhysics?)))

(event Collision|EventActorEndOverlap
  (params (OtherActor :type Actor%20Object%20Reference))
  (Input|DisableInput (Game|GetPlayerController 0))
  (bind _asbp_aria_character_2 (Utilities|Casting|CastToBP_AriaCharacter2 OtherActor))
  (Variables|Default|SetESlate_Visibility "Hidden")
  (Default|GetInformationName _asbp_aria_character_2 (Variables|Default|GetActorReference))
  (Utilities|FlowControl|Gate true) ; enters at Close
)

(event Input|ActionEvents|InputActionInteract
  (params (Key :type Key%20Structure :default "None"))
  (:Pressed
    (Utilities|FlowControl|Gate true
      (:Exit
        (if (Utilities|DoesObjectImplementInterface (stale Collision|EventActorBeginOverlap OtherActor) "/Game/TerraHyphea/World_Level/Blueprints/PickUpItem_Interface.PickUpItem_Interface_C")
          (if (not (Utilities|ClassIsChildOf (Utilities|GetClass (stale Collision|EventActorBeginOverlap OtherActor)) "B_ItemPickupParent_C"))
            (bind _succes (Default|AddtoInventory (Variables|/Game/TerraHyphea/World_Level/Blueprints/BP_AriaCharacter2.BP_AriaCharacter2_C|GetInventoryComponent (stale Collision|EventActorBeginOverlap _asbp_aria_character_2)) (Utilities|GetClass self) 1))
            (if _succes
              (bind _asbp_aria_character_2 (Utilities|Casting|CastToBP_AriaCharacter2 (stale Collision|EventActorBeginOverlap OtherActor)))
              (Default|RefreshInventory (Variables|/Game/TerraHyphea/World_Level/Blueprints/Pickup_Items/W_HeadsUpDisplay.W_HeadsUpDisplay_C|GetW_InventoryBag (Variables|/Game/TerraHyphea/World_Level/Blueprints/BP_AriaCharacter2.BP_AriaCharacter2_C|GetHeadsUpDisplay _asbp_aria_character_2)))
              (CallFunction|PlayPickupSounds (Variables|Default|GetFMODSound))
              (Actor|DestroyActor))))))))

(fn ConstructionScript)

(fn PlayPickupSounds
  (params (Pickup%20Sound :type FMOD%20Event%20Object%20Reference))
  (Class|FMODBlueprintStatics|PlayEventatLocation Pickup%20Sound (Math|Conversions|ToTransform(Vector) (Transformation|GetActorLocation (Game|GetPlayerController 0)))))

(fn GetInformation
  (return (Variables|Default|GetInformation)))

(fn GetPickupItemData
  (return 0 0 0))

(fn GetVisibility
  (return (Variables|Default|GetESlate_Visibility)))

(fn PickupItem
  (params (ItemClass :type Actor%20Class%20Reference) (Itemicon :type Texture%202D%20Object%20Reference) (StackAmount :type Integer))
  (return))