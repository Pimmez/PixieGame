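; B_FiberGrass is a harvestable grass actor that the player hits with left click to get a fiber pickup actor.
; Overlap by a BP_ThirdPersonCharacter with a weapon enables input, opens a click gate and passes itself to GetInformationName; leaving reverses the input and gate.
; Each click decrements Health and plays a Grass sound event at the player.
; A click at zero Health spawns B_ChildFiber and destroys the grass.
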(event EventBeginPlay
  (Variables|Default|SetActor%20Reference self))

(event Collision|EventActorBeginOverlap
  (params (OtherActor :type Actor%20Object%20Reference))
  (bind _asbp_third_person_character (Utilities|Casting|CastToBP_ThirdPersonCharacter OtherActor))
  (Default|HasWeaponEvent _asbp_third_person_character)
  (if (Variables|/Game/ThirdPartyAssets/ThirdPerson/Blueprints/BP_ThirdPersonCharacter.BP_ThirdPersonCharacter_C|GetHasWeapon? _asbp_third_person_character)
    (Variables|Default|SetESlate_Visibility "Hidden")
    (Default|GetInformationName _asbp_third_person_character (Variables|Default|GetActor%20Reference))
    (Input|EnableInput (Game|GetPlayerController 0))
    (Utilities|FlowControl|Gate true) ; enters at Open
  ))

(event EventTick
  (params (DeltaSeconds :type Float%20%28single-precision%29)))

(event Collision|EventActorEndOverlap
  (params (OtherActor :type Actor%20Object%20Reference))
  (bind _asbp_third_person_character (Utilities|Casting|CastToBP_ThirdPersonCharacter OtherActor))
  (Variables|Default|SetESlate_Visibility "Hidden")
  (Default|GetInformationName _asbp_third_person_character (Variables|Default|GetActor%20Reference))
  (Input|DisableInput (Game|GetPlayerController 0))
  (Utilities|FlowControl|Gate true) ; enters at Close
)

(event Input|MouseEvents|LeftMouseButton
  (params (Key :type Key%20Structure :default "None"))
  (:Pressed
    (Utilities|FlowControl|Gate true
      (:Exit
        (Development|PrintString "Hello")
        (if (<= (Variables|Default|GetHealth) 0)
          (Game|SpawnActorfromClass "/Game/TerraHyphea/World_Level/Blueprints/Pickup_Items/B_ChildFiber.B_ChildFiber_C" (Math|Conversions|ToTransform(Vector) (Transformation|GetActorLocation)) "Undefined" 0 0)
          (Actor|DestroyActor)
          (else
            (Math|Integer|DecrementInt (Variables|Default|GetHealth)
              (:%20%20
                (Class|FMODBlueprintStatics|PlayEventatLocation "/Game/FMOD/Events/Combat/Attacks/Impacts/Grass.Grass" (Math|Conversions|ToTransform(Vector) (Transformation|GetActorLocation (Game|GetPlayerCharacter 0))))))))))))

(fn ConstructionScript)

(fn GetInformation
  (return (Variables|Default|GetInformation)))

(fn GetVisibility
  (return (Variables|Default|GetESlate_Visibility)))