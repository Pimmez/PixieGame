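; B_CraftingStone is a world crafting station that spawns a craftable item once when the player has enough stack.
; Overlapping BP_AriaCharacter2 opens a gate, enables input and passes prompt text and visibility through getter functions.
; Interact loops over inventory widgets, but the class check changes nothing, so the last stack amount is compared to CraftingAmount.
; Success spawns at SpawnPoint and disables sphere overlaps; failure shows a find-stones message.
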(event EventBeginPlay
  (Variables|Default|SetActor%20Reference self))

(event Collision|EventActorBeginOverlap
  (params (OtherActor :type Actor%20Object%20Reference))
  (bind _asbp_aria_character_2 (Utilities|Casting|CastToBP_AriaCharacter2 OtherActor))
  (Variables|Default|SetESlate_Visibility "Visible")
  (Variables|Default|SetInformation "Craft")
  (Default|GetInformationName _asbp_aria_character_2 (Variables|Default|GetActor%20Reference))
  (Input|EnableInput (Game|GetPlayerController 0))
  (Utilities|FlowControl|Gate true) ; enters at Open
)

(event Collision|EventActorEndOverlap
  (params (OtherActor :type Actor%20Object%20Reference))
  (bind _asbp_aria_character_2 (Utilities|Casting|CastToBP_AriaCharacter2 OtherActor))
  (Variables|Default|SetESlate_Visibility "Hidden")
  (Variables|Default|SetInformation "")
  (Default|GetInformationName _asbp_aria_character_2 (Variables|Default|GetActor%20Reference))
  (Input|DisableInput (Game|GetPlayerController 0))
  (Utilities|FlowControl|Gate true) ; enters at Close
)

(event Input|ActionEvents|InputActionInteract
  (params (Key :type Key%20Structure :default "None"))
  (:Pressed
    (Utilities|FlowControl|Gate true
      (:Exit
        (bind _array_element (Utilities|Array|ForEachLoopwithBreak (Class|PanelWidget|GetAllChildren (Variables|/Game/TerraHyphea/Demo_Level/Blueprints/UI/W_Inventory.W_Inventory_C|GetInventoryBox (Variables|/Game/TerraHyphea/World_Level/Blueprints/BP_AriaCharacter2.BP_AriaCharacter2_C|GetInventoryWidget (stale Collision|EventActorBeginOverlap _asbp_aria_character_2)))))
          (:LoopBody
            (bind (_itemclass _currentstackamount) (Class|PickUpItemInterface|GetPickupItemData(Message) _array_element))
            (if (== _itemclass (Variables|Default|GetCraftableIngredient))
              _
              (else
                _))
            (Variables|Default|SetInventoryAmount _currentstackamount))
          (:Completed
            (if (>= (Variables|Default|GetInventoryAmount) (Variables|Default|GetCraftingAmount))
              (Utilities|FlowControl|DoOnce false
                (:Completed
                  (Variables|Default|SetInformation "Sword Crafted!")
                  (Default|GetInformationName (stale Collision|EventActorBeginOverlap _asbp_aria_character_2) (Variables|Default|GetActor%20Reference))
                  (bind _returnvalue (Game|SpawnActorfromClass (Variables|Default|GetCraftableItem) (Math|Transform|MakeTransform (Transformation|GetWorldLocation (Variables|Default|GetSpawnPoint))) "Undefined" 0 0))
                  (Utilities|IsValid _returnvalue
                    (:Is%20Valid
                      (Variables|/Script/Engine.PrimitiveComponent|SetbGenerateOverlapEvents (Variables|Default|GetSphereOverlap) false)))))
              (else
                (Variables|Default|SetInformation "Find 2 Stones!")
                (Default|GetInformationName (stale Collision|EventActorBeginOverlap _asbp_aria_character_2) (Variables|Default|GetActor%20Reference))))))))))

(fn ConstructionScript)

(fn GetInformation
  (return (Variables|Default|GetInformation)))

(fn GetPickupItemData
  (return 0 0 0))

(fn GetVisibility
  (return (Variables|Default|GetESlate_Visibility)))