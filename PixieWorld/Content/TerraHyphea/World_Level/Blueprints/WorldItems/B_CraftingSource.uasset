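; B_CraftingSource is a world crafting station that opens the crafting HUD when Aria interacts while overlapping it.
; Overlap enables input and opens a Gate; Interact then disables her movement, adds W_CraftingHUD and switches to Game-and-UI input with a cursor.
; Getters expose prompt text and visibility.
; Older prompt, inventory-check and item-spawn logic is disconnected, leaving a second Interact gate inert.
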(event EventBeginPlay
  (Variables|Default|SetActor%20Reference self))

(event Collision|EventActorBeginOverlap
  (params (OtherActor :type Actor%20Object%20Reference))
  (bind _returnvalue (Game|GetPlayerController 0))
  (bind _asbp_aria_character_2 (Utilities|Casting|CastToBP_AriaCharacter2 OtherActor))
  (Input|EnableInput (Game|GetPlayerController 0))
  (Utilities|FlowControl|Gate true) ; enters at Open
)

(event Collision|EventActorEndOverlap
  (params (OtherActor :type Actor%20Object%20Reference))
  (bind _returnvalue (Game|GetPlayerController 0))
  (Utilities|Casting|CastToBP_AriaCharacter2 OtherActor)
  (Input|DisableInput (Game|GetPlayerController 0))
  (Utilities|FlowControl|Gate true) ; enters at Close
)

(event Input|ActionEvents|InputActionInteract
  (params (Key :type Key%20Structure :default "None"))
  (bind _returnvalue (Game|GetPlayerController 0))
  (:Pressed
    (Utilities|FlowControl|Gate true
      (:Exit
        (Pawn|Components|CharacterMovement|DisableMovement (Variables|/Script/Engine.Character|GetCharacterMovement (stale Collision|EventActorBeginOverlap _asbp_aria_character_2)))
        (bind _returnvalue_2 (UserInterface|CreateWidget "/Game/TerraHyphea/World_Level/Blueprints/UI/W_CraftingHUD.W_CraftingHUD_C"))
        (bind _output_get (Variables|Default|SetSetCraftingWidget _returnvalue_2))
        (UserInterface|Viewport|AddtoViewport _output_get 0)
        (Input|SetInputModeGameandUI _returnvalue 0 "DoNotLock" true)
        (Variables|/Script/Engine.PlayerController|SetbShowMouseCursor _returnvalue true)))))

(event Input|ActionEvents|InputActionInteract
  (params (Key :type Key%20Structure :default "None"))
  (:Pressed
    (Utilities|FlowControl|Gate true)))

(fn ConstructionScript)

(fn GetInformation
  (return (Variables|Default|GetInformation)))

(fn GetPickupItemData
  (return 0 0 0))

(fn GetVisibility
  (return (Variables|Default|GetESlate_Visibility)))