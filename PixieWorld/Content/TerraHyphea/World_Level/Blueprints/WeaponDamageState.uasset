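; WeaponDamageState is an animation notify state that marks the window in an animation when Aria's weapon is active, likely for dealing damage.
; On begin and end, it casts the mesh owner to BP_AriaCharacter2 and its child actor to BP_BaseWeaponItem.
; It then calls WeaponActive at the start of the window and WeaponDeactivate at the end, doing nothing if either cast fails.
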(fn ReceivedNotifyBegin
  (params (MeshComp :type Skeletal%20Mesh%20Component%20Object%20Reference) (Animation :type Anim%20Sequence%20Base%20Object%20Reference) (TotalDuration :type Float%20%28single-precision%29) (EventReference :type Anim%20Notify%20Event%20Reference%20Structure%20%28by%20ref%29))
  (bind _asbp_aria_character_2 (Utilities|Casting|CastToBP_AriaCharacter2 (Components|GetOwner MeshComp)))
  (bind _asbp_base_weapon_item (Utilities|Casting|CastToBP_BaseWeaponItem (Variables|/Script/Engine.ChildActorComponent|GetChildActor (Variables|/Game/TerraHyphea/World_Level/Blueprints/BP_AriaCharacter2.BP_AriaCharacter2_C|GetChildActor _asbp_aria_character_2))))
  (Default|WeaponActive _asbp_base_weapon_item)
  (return false))

(fn ReceivedNotifyEnd
  (params (MeshComp :type Skeletal%20Mesh%20Component%20Object%20Reference) (Animation :type Anim%20Sequence%20Base%20Object%20Reference) (EventReference :type Anim%20Notify%20Event%20Reference%20Structure%20%28by%20ref%29))
  (bind _asbp_aria_character_2 (Utilities|Casting|CastToBP_AriaCharacter2 (Components|GetOwner MeshComp)))
  (bind _asbp_base_weapon_item (Utilities|Casting|CastToBP_BaseWeaponItem (Variables|/Script/Engine.ChildActorComponent|GetChildActor (Variables|/Game/TerraHyphea/World_Level/Blueprints/BP_AriaCharacter2.BP_AriaCharacter2_C|GetChildActor _asbp_aria_character_2))))
  (Default|WeaponDeactivate _asbp_base_weapon_item)
  (return false))