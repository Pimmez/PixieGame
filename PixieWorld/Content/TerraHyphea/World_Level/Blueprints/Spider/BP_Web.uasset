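; Spider boss web with three breakable pillars, each with its own health and sparkle effect.
; Every overlap on a pillar plays a hit sound at the player and decrements its health, or breaks it if health is already depleted.
; Breaking a pillar removes it and its sparkle and sets HasWebPieceBroken? on the BP_SpiderBoss blackboard.
; The third break destroys the whole web instead, without setting that flag.
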(event OnComponentBeginOverlap(Pillar1)
  (params (OverlappedComponent :type Primitive%20Component%20Object%20Reference) (OtherActor :type Actor%20Object%20Reference) (OtherComp :type Primitive%20Component%20Object%20Reference) (OtherBodyIndex :type Integer) (bFromSweep :type Boolean) (SweepResult :type Hit%20Result%20Structure%20%28by%20ref%29))
  (bind _pillar1health (Variables|Default|GetPillar1Health))
  (Class|FMODBlueprintStatics|PlayEventatLocation "/Game/FMOD/Events/Combat/Attacks/Impacts/Web_Hit.Web_Hit" (Math|Conversions|ToTransform(Vector) (Transformation|GetActorLocation (Game|GetPlayerCharacter 0))))
  (if (<= _pillar1health 0.0)
    (bind _result (Math|Integer|IncrementInt (Variables|Default|GetIncrementDeathCounter))
      (:%20%20
        (if (== _result 3)
          (Actor|DestroyActor)
          (else
            (Components|DestroyComponent (Variables|Default|GetPillar1))
            (Components|DestroyComponent (Variables|Default|GetNS_Sparkle_3))
            (bind _outactors (Actor|GetAllActorsOfClass "/Game/TerraHyphea/World_Level/Blueprints/Spider/BP_SpiderBoss.BP_SpiderBoss_C"))
            (AI|Components|Blackboard|SetValueasBool (AI|GetBlackboard (AI|GetAIController (Utilities|Array|Get(acopy) _outactors))) (Utilities|Name|MakeLiteralName "HasWebPieceBroken?") true)))))
    (else
      (bind _result_2 (Math|Float|DecrementFloat _pillar1health)
        (:%20%20
          (Development|PrintString (Utilities|String|ToString(Float) _result_2)))))))

(event OnComponentBeginOverlap(Pillar2)
  (params (OverlappedComponent :type Primitive%20Component%20Object%20Reference) (OtherActor :type Actor%20Object%20Reference) (OtherComp :type Primitive%20Component%20Object%20Reference) (OtherBodyIndex :type Integer) (bFromSweep :type Boolean) (SweepResult :type Hit%20Result%20Structure%20%28by%20ref%29))
  (bind _pillar2health (Variables|Default|GetPillar2Health))
  (Class|FMODBlueprintStatics|PlayEventatLocation "/Game/FMOD/Events/Combat/Attacks/Impacts/Web_Hit.Web_Hit" (Math|Conversions|ToTransform(Vector) (Transformation|GetActorLocation (Game|GetPlayerCharacter 0))))
  (if (<= _pillar2health 0.0)
    (bind _result (Math|Integer|IncrementInt (Variables|Default|GetIncrementDeathCounter))
      (:%20%20
        (if (== _result 3)
          (Actor|DestroyActor)
          (else
            (Components|DestroyComponent (Variables|Default|GetPillar2))
            (Components|DestroyComponent (Variables|Default|GetNS_Sparkle_2))
            (bind _outactors (Actor|GetAllActorsOfClass "/Game/TerraHyphea/World_Level/Blueprints/Spider/BP_SpiderBoss.BP_SpiderBoss_C"))
            (AI|Components|Blackboard|SetValueasBool (AI|GetBlackboard (AI|GetAIController (Utilities|Array|Get(acopy) _outactors))) (Utilities|Name|MakeLiteralName "HasWebPieceBroken?") true)))))
    (else
      (bind _result_2 (Math|Float|DecrementFloat _pillar2health)
        (:%20%20
          (Development|PrintString (Utilities|String|ToString(Float) _result_2)))))))

(event OnComponentBeginOverlap(Pillar3)
  (params (OverlappedComponent :type Primitive%20Component%20Object%20Reference) (OtherActor :type Actor%20Object%20Reference) (OtherComp :type Primitive%20Component%20Object%20Reference) (OtherBodyIndex :type Integer) (bFromSweep :type Boolean) (SweepResult :type Hit%20Result%20Structure%20%28by%20ref%29))
  (bind _pillar3health (Variables|Default|GetPillar3Health))
  (Class|FMODBlueprintStatics|PlayEventatLocation "/Game/FMOD/Events/Combat/Attacks/Impacts/Web_Hit.Web_Hit" (Math|Conversions|ToTransform(Vector) (Transformation|GetActorLocation (Game|GetPlayerCharacter 0))))
  (if (<= _pillar3health 0.0)
    (bind _result (Math|Integer|IncrementInt (Variables|Default|GetIncrementDeathCounter))
      (:%20%20
        (if (== _result 3)
          (Actor|DestroyActor)
          (else
            (Components|DestroyComponent (Variables|Default|GetPillar3))
            (Components|DestroyComponent (Variables|Default|GetNS_Sparkle_4))
            (bind _outactors (Actor|GetAllActorsOfClass "/Game/TerraHyphea/World_Level/Blueprints/Spider/BP_SpiderBoss.BP_SpiderBoss_C"))
            (AI|Components|Blackboard|SetValueasBool (AI|GetBlackboard (AI|GetAIController (Utilities|Array|Get(acopy) _outactors))) (Utilities|Name|MakeLiteralName "HasWebPieceBroken?") true)))))
    (else
      (bind _result_2 (Math|Float|DecrementFloat _pillar3health)
        (:%20%20
          (Development|PrintString (Utilities|String|ToString(Float) _result_2)))))))

(event EventBeginPlay)

(fn ConstructionScript)