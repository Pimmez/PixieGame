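; Spider boss that detects the player character Aria and can fire slime projectiles at her.
; Pawn sensing sets the "HasSeenPlayer?" key on its AI controller's blackboard.
; ShootProjectile spawns a slime projectile at Arrow1, rotated toward the player reference cached at BeginPlay.
; Tick polls the Isded flag, then plays the Blob_Death event at the boss's location and destroys the actor.
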(event OnSeePawn(PawnSensing)
  (params (Pawn :type Pawn%20Object%20Reference))
  (Utilities|Casting|CastToBP_AriaCharacter2 Pawn)
  (AI|Components|Blackboard|SetValueasBool (AI|GetBlackboard (AI|GetAIController self)) (Utilities|Name|MakeLiteralName "HasSeenPlayer?") true))

(event EventBeginPlay
  (bind _asbp_aria_character_2 (Utilities|Casting|CastToBP_AriaCharacter2 (Game|GetPlayerCharacter 0)))
  (Variables|Default|SetAs%20BP%20Aria%20Character%202 _asbp_aria_character_2))

(event EventTick
  (params (DeltaSeconds :type Float%20%28single-precision%29))
  (if (Variables|Default|Getisded)
    (Class|FMODBlueprintStatics|PlayEventatLocation "/Game/FMOD/Events/Blob_Death.Blob_Death" (Math|Conversions|ToTransform(Vector) (Transformation|GetActorLocation)))
    (Actor|DestroyActor)))

(fn ConstructionScript)

(fn ShootProjectile
  (bind _arrow1 (Variables|Default|GetArrow1))
  (bind _returnvalue (Transformation|GetWorldLocation _arrow1))
  (Game|SpawnActorfromClass "/Game/TerraHyphea/World_Level/Blueprints/Spider/BP_SlimeProjectile.BP_SlimeProjectile_C" (Math|Transform|MakeTransform _returnvalue (Math|Rotator|FindLookatRotation _returnvalue (Transformation|GetActorLocation (Variables|Default|GetAs%20BP%20Aria%20Character%202))) "1.000000,1.000000,1.000000") "Undefined" 0 0))