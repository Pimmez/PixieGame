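; Behavior tree task that makes the spider boss spawn a wave of slime enemies.
; It plays the Blob_Spawn audio event at the player's location, then loops EnemySpawned times, spawning slimes at the boss's three spawn points.
; The first three indices map to points A, B and C, and any further ones fall back to A.
; It then resets EnemySpawned to EnemyIncrement plus a fixed base and finishes successfully.
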(event EventReceiveExecuteAI
  (params (OwnerController :type AI%20Controller%20Object%20Reference) (ControlledPawn :type Pawn%20Object%20Reference))
  (bind _asbp_spider_boss (Utilities|Casting|CastToBP_SpiderBoss ControlledPawn))
  (Class|FMODBlueprintStatics|PlayEventatLocation "/Game/FMOD/Events/Combat/Enemies/Blob/Blob_Spawn.Blob_Spawn" (Math|Conversions|ToTransform(Vector) (Transformation|GetActorLocation (Game|Player|GetPlayerPawn 0))))
  (for _index (range 0 (- (Variables|Default|GetEnemySpawned) 1))
    (switch int _index
      (:Default
        (Game|SpawnActorfromClass "/Game/TerraHyphea/World_Level/Blueprints/BP_Enemy/BP_EnemySlime.BP_EnemySlime_C" (Math|Conversions|ToTransform(Vector) (Transformation|GetWorldLocation (Variables|/Game/TerraHyphea/World_Level/Blueprints/Spider/BP_SpiderBoss.BP_SpiderBoss_C|GetSpawnLocationA _asbp_spider_boss))) "Undefined" 0 0 :!label _label))
      (:0
        (goto _label))
      (:1
        (Game|SpawnActorfromClass "/Game/TerraHyphea/World_Level/Blueprints/BP_Enemy/BP_EnemySlime.BP_EnemySlime_C" (Math|Conversions|ToTransform(Vector) (Transformation|GetWorldLocation (Variables|/Game/TerraHyphea/World_Level/Blueprints/Spider/BP_SpiderBoss.BP_SpiderBoss_C|GetSpawnLocationB _asbp_spider_boss))) "Undefined" 0 0))
      (:2
        (Game|SpawnActorfromClass "/Game/TerraHyphea/World_Level/Blueprints/BP_Enemy/BP_EnemySlime.BP_EnemySlime_C" (Math|Conversions|ToTransform(Vector) (Transformation|GetWorldLocation (Variables|/Game/TerraHyphea/World_Level/Blueprints/Spider/BP_SpiderBoss.BP_SpiderBoss_C|GetSpawnLocationC _asbp_spider_boss))) "Undefined" 0 0))))
  (Variables|Default|SetEnemySpawned (+ (Variables|Default|GetEnemyIncrement) 3))
  (AI|BehaviorTree|FinishExecute true))