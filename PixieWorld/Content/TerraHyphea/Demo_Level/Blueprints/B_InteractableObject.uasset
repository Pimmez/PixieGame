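; Interactable planting spot that turns mushroom seeds into a bounce pad launching the player upward with pitch-randomized sound.
; Character overlap shows a prompt, enables input and opens a gate; Interact scans the inventory widget's children for stack amounts.
; The item-class check has no effect, so the last stack read decides.
; A nonzero amount reveals the hidden meshes and enables the launch overlap; otherwise a find-seeds message appears.
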(event OnComponentBeginOverlap(StaticMesh1)
  (params (OverlappedComponent :type Primitive%20Component%20Object%20Reference) (OtherActor :type Actor%20Object%20Reference) (OtherComp :type Primitive%20Component%20Object%20Reference) (OtherBodyIndex :type Integer) (bFromSweep :type Boolean) (SweepResult :type Hit%20Result%20Structure%20%28by%20ref%29))
  (bind _returnvalue (Math|Random|RandomFloatinRange 0.8 1.3))
  (bind _returnvalue_2 (Game|GetPlayerCharacter 0))
  (bind _returnvalue_3 (Transformation|GetActorLocation _returnvalue_2))
  (Utilities|IsValid _returnvalue_2
    (:Is%20Valid
      (Character|LaunchCharacter _returnvalue_2 "0, 0,2000.000000" false true)
      (Audio|PlaySoundatLocation 0 _returnvalue_3 "0, 0, 0" 1.0 _returnvalue 0.0 0 0 0 0)
      (Audio|PlaySoundatLocation 0 _returnvalue_3 "0, 0, 0" 1.0 _returnvalue 0.0 0 0 0 0))))

(event EventBeginPlay
  (bind _staticmesh (Variables|Default|GetStaticMesh))
  (Rendering|SetVisibility _staticmesh false false)
  (Collision|SetCollisionEnabled _staticmesh "NoCollision"))

(event Collision|EventActorBeginOverlap
  (params (OtherActor :type Actor%20Object%20Reference))
  (bind _staticmesh (Variables|Default|GetStaticMesh))
  (bind _asbp_third_person_character (Utilities|Casting|CastToBP_ThirdPersonCharacter OtherActor))
  (Variables|Default|SetInformation "Press F to Plant")
  (Default|GetInformationName _asbp_third_person_character (Variables|Default|GetActor%20Reference))
  (Input|EnableInput (Game|GetPlayerController 0))
  (bind _asbp_third_person_character_2 (Utilities|Casting|CastToBP_ThirdPersonCharacter OtherActor))
  (Utilities|FlowControl|Gate true) ; enters at Open
)

(event Collision|EventActorEndOverlap
  (params (OtherActor :type Actor%20Object%20Reference))
  (bind _asbp_third_person_character (Utilities|Casting|CastToBP_ThirdPersonCharacter OtherActor))
  (Variables|Default|SetInformation "")
  (Default|GetInformationName _asbp_third_person_character)
  (Input|DisableInput 0))

(event Input|ActionEvents|InputActionInteract
  (params (Key :type Key%20Structure))
  (bind _staticmesh (Variables|Default|GetStaticMesh))
  (:Pressed
    (Utilities|FlowControl|Gate true
      (:Exit
        (bind _array_element (Utilities|Array|ForEachLoopwithBreak (Class|PanelWidget|GetAllChildren (Variables|/Game/TerraHyphea/Demo_Level/Blueprints/UI/W_Inventory.W_Inventory_C|GetInventoryBox (Variables|/Game/ThirdPartyAssets/ThirdPerson/Blueprints/BP_ThirdPersonCharacter.BP_ThirdPersonCharacter_C|GetInventoryWidget (stale Collision|EventActorBeginOverlap _asbp_third_person_character_2)))))
          (:LoopBody
            (bind (_itemclass _currentstackamount) (Class|PickUpItemInterface|GetPickupItemData(Message) _array_element))
            (if (== _itemclass (Variables|Default|GetItemToUse))
              _
              (else
                _))
            (Variables|Default|SetInventoryAmount _currentstackamount))
          (:Completed
            (if (>= (Variables|Default|GetInventoryAmount) 1)
              (Variables|Default|SetInformation "Seeds Planted!")
              (Default|GetInformationName (stale Collision|EventActorBeginOverlap _asbp_third_person_character_2) (Variables|Default|GetActor%20Reference))
              (Rendering|SetVisibility _staticmesh true false)
              (Collision|SetCollisionEnabled _staticmesh "QueryAndPhysics")
              (Variables|/Script/Engine.PrimitiveComponent|SetbGenerateOverlapEvents (Variables|Default|GetStaticMesh1) true)
              (Variables|/Script/Engine.PrimitiveComponent|SetbGenerateOverlapEvents (Variables|Default|GetOverlapSphere) false)
              (else
                (Variables|Default|SetInformation "Find Mushrooms Seeds!")
                (Default|GetInformationName (stale Collision|EventActorBeginOverlap _asbp_third_person_character_2) (Variables|Default|GetActor%20Reference))))))))))

(fn ConstructionScript)

(fn GetInformation
  (return (Variables|Default|GetInformation)))

(fn GetPickupItemData
  (return 0 0 0))