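; B_Grass_01 is a cuttable grass actor for the TerraHyphea demo level that the player damages with left mouse clicks.
; Overlap by an armed third-person character passes it info, enables input and opens a gate; leaving clears these.
; Each click through the gate decrements Health and plays two sounds at the player's location.
; Tick destroys the actor once Health runs out, and GetInformation returns its Information.
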(event Collision|EventActorBeginOverlap
  (params (OtherActor :type Actor%20Object%20Reference))
  (bind _returnvalue (Game|GetPlayerCharacter 0))
  (bind _returnvalue_2 (Transformation|GetActorLocation _returnvalue))
  (bind _asbp_third_person_character (Utilities|Casting|CastToBP_ThirdPersonCharacter OtherActor))
  (Default|HasWeaponEvent _asbp_third_person_character)
  (if (Variables|/Game/ThirdPartyAssets/ThirdPerson/Blueprints/BP_ThirdPersonCharacter.BP_ThirdPersonCharacter_C|GetHasWeapon? _asbp_third_person_character)
    (Default|GetInformationName _asbp_third_person_character (Variables|Default|GetActor%20Reference))
    (Input|EnableInput (Game|GetPlayerController 0))
    (Utilities|FlowControl|Gate true) ; enters at Open
  ))

(event EventTick
  (params (DeltaSeconds :type Float%20%28single-precision%29))
  (if (<= (Variables|Default|GetHealth) 0)
    (Actor|DestroyActor)))

(event Collision|EventActorEndOverlap
  (params (OtherActor :type Actor%20Object%20Reference))
  (bind _returnvalue (Game|GetPlayerCharacter 0))
  (bind _returnvalue_2 (Transformation|GetActorLocation _returnvalue))
  (bind _asbp_third_person_character (Utilities|Casting|CastToBP_ThirdPersonCharacter OtherActor))
  (Default|GetInformationName _asbp_third_person_character)
  (Input|DisableInput (Game|GetPlayerController 0))
  (Utilities|FlowControl|Gate true) ; enters at Close
)

(event Input|MouseEvents|LeftMouseButton
  (params (Key :type Key%20Structure))
  (bind _returnvalue (Game|GetPlayerCharacter 0))
  (bind _returnvalue_2 (Transformation|GetActorLocation _returnvalue))
  (:Pressed
    (Utilities|FlowControl|Gate true
      (:Exit
        (Math|Integer|DecrementInt (Variables|Default|GetHealth)
          (:%20%20
            (Audio|PlaySoundatLocation 0 _returnvalue_2 "0, 0, 0" 1.0 1.0 0.0 0 0 0 0)
            (Audio|PlaySoundatLocation 0 _returnvalue_2 "0, 0, 0" 1.2 1.0 0.0 0 0 0 0)))))))

(fn ConstructionScript)

(fn GetInformation
  (return (Variables|Default|GetInformation)))