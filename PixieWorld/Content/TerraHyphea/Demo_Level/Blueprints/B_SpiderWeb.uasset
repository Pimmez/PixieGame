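; Destructible spider web obstacle with left and right halves that the player breaks by left-clicking while carrying a weapon.
; Each overlap sphere enables input and opens a gate for its side, passing the web to the character's information function.
; Clicks lower that side's health with a hit sound and remove its box at zero, after a delay on the left.
; Tick destroys the actor with a sound once both sides reach zero.
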(event OnComponentBeginOverlap(SphereOverlap_R)
  (params (OverlappedComponent :type Primitive%20Component%20Object%20Reference) (OtherActor :type Actor%20Object%20Reference) (OtherComp :type Primitive%20Component%20Object%20Reference) (OtherBodyIndex :type Integer) (bFromSweep :type Boolean) (SweepResult :type Hit%20Result%20Structure%20%28by%20ref%29))
  (bind _health_r (Variables|Default|GetHealth_R))
  (bind _asbp_third_person_character (Utilities|Casting|CastToBP_ThirdPersonCharacter OtherActor))
  (Variables|Default|SetESlate_Visibility "Hidden")
  (if (Variables|/Game/ThirdPartyAssets/ThirdPerson/Blueprints/BP_ThirdPersonCharacter.BP_ThirdPersonCharacter_C|GetHasWeapon? _asbp_third_person_character)
    (Default|GetInformationName _asbp_third_person_character (Variables|Default|GetActor%20Reference))
    (Input|EnableInput (Game|GetPlayerController 0))
    (Utilities|FlowControl|Gate true) ; enters at Open
  ))

(event OnComponentBeginOverlap(SphereOverlap_L)
  (params (OverlappedComponent :type Primitive%20Component%20Object%20Reference) (OtherActor :type Actor%20Object%20Reference) (OtherComp :type Primitive%20Component%20Object%20Reference) (OtherBodyIndex :type Integer) (bFromSweep :type Boolean) (SweepResult :type Hit%20Result%20Structure%20%28by%20ref%29))
  (bind _health_l (Variables|Default|GetHealth_L))
  (bind _asbp_third_person_character (Utilities|Casting|CastToBP_ThirdPersonCharacter OtherActor))
  (Variables|Default|SetESlate_Visibility "Hidden")
  (if (Variables|/Game/ThirdPartyAssets/ThirdPerson/Blueprints/BP_ThirdPersonCharacter.BP_ThirdPersonCharacter_C|GetHasWeapon? _asbp_third_person_character)
    (Default|GetInformationName _asbp_third_person_character (Variables|Default|GetActor%20Reference))
    (Input|EnableInput (Game|GetPlayerController 0))
    (Utilities|FlowControl|Gate true) ; enters at Open
  ))

(event OnComponentEndOverlap(SphereOverlap_L)
  (params (OverlappedComponent :type Primitive%20Component%20Object%20Reference) (OtherActor :type Actor%20Object%20Reference) (OtherComp :type Primitive%20Component%20Object%20Reference) (OtherBodyIndex :type Integer))
  (bind _health_l (Variables|Default|GetHealth_L))
  (bind _asbp_third_person_character (Utilities|Casting|CastToBP_ThirdPersonCharacter OtherActor))
  (Variables|Default|SetESlate_Visibility "Hidden")
  (Variables|Default|SetInformation "")
  (Default|GetInformationName (stale OnComponentBeginOverlap(SphereOverlap_L) _asbp_third_person_character) (Variables|Default|GetActor%20Reference))
  (Input|DisableInput (Game|GetPlayerController 0))
  (Utilities|FlowControl|Gate true) ; enters at Close
)

(event OnComponentEndOverlap(SphereOverlap_R)
  (params (OverlappedComponent :type Primitive%20Component%20Object%20Reference) (OtherActor :type Actor%20Object%20Reference) (OtherComp :type Primitive%20Component%20Object%20Reference) (OtherBodyIndex :type Integer))
  (bind _health_r (Variables|Default|GetHealth_R))
  (bind _asbp_third_person_character (Utilities|Casting|CastToBP_ThirdPersonCharacter OtherActor))
  (Variables|Default|SetESlate_Visibility "Hidden")
  (Variables|Default|SetInformation "")
  (Default|GetInformationName (stale OnComponentBeginOverlap(SphereOverlap_R) _asbp_third_person_character) (Variables|Default|GetActor%20Reference))
  (Input|DisableInput (Game|GetPlayerController 0))
  (Utilities|FlowControl|Gate true) ; enters at Close
)

(event EventBeginPlay
  (Variables|Default|SetHealth_L 2)
  (Variables|Default|SetHealth_R 2))

(event EventTick
  (params (DeltaSeconds :type Float%20%28single-precision%29))
  (if (and (<= (Variables|Default|GetHealth_L) 0) (<= (Variables|Default|GetHealth_R) 0))
    (Utilities|FlowControl|DoOnce false
      (:Completed
        (Class|FMODBlueprintStatics|PlayEventatLocation "/Game/FMOD/Events/Attacks/Web_Destroy.Web_Destroy" (Math|Conversions|ToTransform(Vector) (Transformation|GetActorLocation (Game|GetPlayerController 0))))
        (Actor|DestroyActor)))))

(event Input|MouseEvents|LeftMouseButton
  (params (Key :type Key%20Structure :default "None"))
  (bind _health_l (Variables|Default|GetHealth_L))
  (:Pressed
    (Utilities|FlowControl|Gate true :!label _label
      (:Exit
        (Math|Integer|DecrementInt _health_l
          (:%20%20
            (Class|FMODBlueprintStatics|PlayEventatLocation "/Game/FMOD/Events/Attacks/Web_Hit.Web_Hit" (Math|Conversions|ToTransform(Vector) (Transformation|GetActorLocation (Game|GetPlayerController 0))))
            (if (<= _health_l 0)
              (Utilities|FlowControl|Delay 1.0)
              (Components|DestroyComponent (Variables|Default|Getbox1))
              (goto _label Close))))))))

(event Input|MouseEvents|LeftMouseButton
  (params (Key :type Key%20Structure :default "None"))
  (bind _health_r (Variables|Default|GetHealth_R))
  (:Pressed
    (Utilities|FlowControl|Gate true :!label _label
      (:Exit
        (Math|Integer|DecrementInt _health_r
          (:%20%20
            (Class|FMODBlueprintStatics|PlayEventatLocation "/Game/FMOD/Events/Attacks/Web_Hit.Web_Hit" (Math|Conversions|ToTransform(Vector) (Transformation|GetActorLocation (Game|GetPlayerController 0))))
            (if (<= _health_r 0)
              (Components|DestroyComponent (Variables|Default|Getbox))
              (goto _label Close))))))))

(fn ConstructionScript)

(fn GetInformation
  (return (Variables|Default|GetInformation)))

(fn GetVisibility
  (return (Variables|Default|GetESlate_Visibility)))