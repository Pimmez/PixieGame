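; B_Slime is a demo-level enemy that damages the overlapping third-person character and can be slashed to death.
; Overlap sets its attacking state and, if the player has a weapon, shares its reference, enables input and opens a Gate.
; Left-clicks through that Gate decrement health and play sounds at the player.
; Tick destroys it at zero health, otherwise uses a Delay to pace attacks to roughly one per second.
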(event Collision|EventActorBeginOverlap
  (params (OtherActor :type Actor%20Object%20Reference))
  (bind _returnvalue (Game|GetPlayerCharacter 0))
  (bind _returnvalue_2 (Transformation|GetActorLocation _returnvalue))
  (bind _asbp_third_person_character (Utilities|Casting|CastToBP_ThirdPersonCharacter OtherActor))
  (Variables|Default|SetIsAttacking? true)
  (Default|HasWeaponEvent _asbp_third_person_character)
  (if (Variables|/Game/ThirdPartyAssets/ThirdPerson/Blueprints/BP_ThirdPersonCharacter.BP_ThirdPersonCharacter_C|GetHasWeapon? _asbp_third_person_character)
    (Default|GetInformationName _asbp_third_person_character (Variables|Default|GetActor%20Reference))
    (Input|EnableInput (Game|GetPlayerController 0))
    (Utilities|FlowControl|Gate true) ; enters at Open
  ))

(event EventTick
  (params (DeltaSeconds :type Float%20%28single-precision%29))
  (if (<= (Variables|Default|Gethealth) 0)
    (Actor|DestroyActor)
    (elif (Variables|Default|GetIsAttacking?)
      (Utilities|FlowControl|Delay 1.0)
      (CallFunction|Attack (stale Collision|EventActorBeginOverlap _asbp_third_person_character)))))

(event Collision|EventActorEndOverlap
  (params (OtherActor :type Actor%20Object%20Reference))
  (bind _returnvalue (Game|GetPlayerCharacter 0))
  (bind _returnvalue_2 (Transformation|GetActorLocation _returnvalue))
  (bind _asbp_third_person_character (Utilities|Casting|CastToBP_ThirdPersonCharacter OtherActor))
  (Variables|Default|SetIsAttacking? false)
  (Default|GetInformationName _asbp_third_person_character)
  (Input|DisableInput (Game|GetPlayerController 0))
  (Utilities|FlowControl|Gate true) ; enters at Close
)

(event Input|MouseEvents|LeftMouseButton
  (params (Key :type Key%20Structure))
  (bind _returnvalue (Game|GetPlayerCharacter 0))
  (bind _returnvalue_2 (Transformation|GetActorLocation _returnvalue))
  (:Pressed
    (Utilities|FlowControl|Gate true
      (:Exit
        (Development|PrintString "SLASH")
        (Math|Integer|DecrementInt (Variables|Default|Gethealth)
          (:%20%20
            (Audio|PlaySoundatLocation 0 _returnvalue_2 "0, 0, 0" 1.0 1.0 0.0 0 0 0 0)
            (Audio|PlaySoundatLocation 0 _returnvalue_2 "0, 0, 0" 1.2 1.0 0.0 0 0 0 0)
            (Audio|PlaySoundatLocation 0 _returnvalue_2 "0, 0, 0" 1.0 1.0 0.0 0 0 0 0)))))))

(fn ConstructionScript)

(fn Attack
  (params (Player%20ref :type BP%20Third%20Person%20Character%20Object%20Reference))
  (Default|DamagePlayer Player%20ref (Variables|Default|GetAttackDamage)))

(fn GetInformation
  (return (Variables|Default|GetInformation)))